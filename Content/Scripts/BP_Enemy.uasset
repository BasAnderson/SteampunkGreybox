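; BP_Enemy is an enemy Blueprint that patrols back and forth between two target points.
; BeginPlay starts the Patrol event, which chains AI MoveTo calls to TargetPoint1 and TargetPoint2 with a short delay after each arrival.
; Patrol calls itself after the second wait to loop.
; A failed move to the first point prints the movement result, while a failed second move is unhandled, so either failure stops the loop.
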(event Custom|Patrol
  (bind _movementresult (AI|AIMoveTo self 0 "0, 0, 0" (Variables|Default|GetTargetPoint1) 5.0 false)
    (:OnSuccess
      (Utilities|FlowControl|Delay 3.0)
      (AI|AIMoveTo self "0, 0, 0" (Variables|Default|GetTargetPoint2) 5.0 false
        (:OnSuccess
          (Utilities|FlowControl|Delay 3.0)
          (CallFunction|Patrol))))
    (:OnFail
      (Development|PrintString (Utilities|String|EnumtoString _movementresult)))))

(event EventBeginPlay
  (CallFunction|Patrol))

(event Collision|EventActorBeginOverlap
  (params (OtherActor :type Actor%20Object%20Reference)))

(event EventTick
  (params (DeltaSeconds :type Float%20%28single-precision%29)))

(fn ConstructionScript)